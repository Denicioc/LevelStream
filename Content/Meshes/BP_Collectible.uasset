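; Collectible actor that removes itself from the level when its Box component registers an overlap.
; The overlap casts the player character to FirstPersonCharacter without checking which actor overlapped, then passes the collectible's display name to W3dGameInstance's ToBeDestroyed.
; It then calls its PickUp event, which destroys the actor.
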(event `self.Box.OnComponentBeginOverlap`
  (params (OverlappedComponent :type "PrimitiveComponent Object Reference") (OtherActor :type "Actor Object Reference") (OtherComp :type "PrimitiveComponent Object Reference") (OtherBodyIndex :type Integer) (bFromSweep :type Boolean) (SweepResult :type "HitResult Structure (by ref)"))
  (set `self.FPSChar` (cast `/Game/FirstPersonBP/Blueprints/FirstPersonCharacter` (`GameplayStatics.GetPlayerCharacter` 0) :!pure true))
  (`/Game/SavedData/W3dGameInstance.ToBeDestroyed` (cast `/Game/SavedData/W3dGameInstance` (`GameplayStatics.GetGameInstance`) :!pure true) (`KismetSystemLibrary.GetDisplayName` self))
  (`self.PickUp`))

(event `PickUp`
  (`self.K2_DestroyActor`))

(fn `UserConstructionScript`)