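; Gatling weapon pickup that bobs and rotates in the world until collected.
; A self-repeating Delay loop from BeginPlay moves the skeletal mesh by small local transforms, with a counter flipping the vertical direction at each limit.
; The PickUp event enables the Gatling and auto fire on the player's FirstPersonCharacter, sets its fire rate, swaps the gun material, then destroys the pickup.
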(event `self.ReceiveBeginPlay`
  (bind _counter (`self.Counter`))
  (bind _counter_2 (`self.Counter`))
  (`SceneComponent.K2_AddLocalTransform` (`self.SkeletalMesh`) (`KismetMathLibrary.MakeTransform` (`KismetMathLibrary.MakeVector` 0.0 0.0 (select `bool` (`self.Floating`) :`false` 0.5 :`true` -0.5 :!type "Float (single-precision)")) (struct :`Yaw` 0.5) (2.0 2.0 2.0)) false false :!label _label)
  (if (== _counter_2 0.0)
    (`|ExecutionSequence`
      (:`then_0`
        (set `self.Floating` false))
      (:`then_1`
        (if (== _counter_2 100.0) :!label _label_2
          (`|ExecutionSequence`
            (:`then_0`
              (set `self.Floating` true))
            (:`then_1`
              (`KismetSystemLibrary.Delay` 0.01 :!label _label_3)
              (if (`self.Floating`)
                (`/Engine/EditorBlueprintResources/StandardMacros.DecrementFloat` _counter
                  (:`  `
                    _))
                (else
                  (`/Engine/EditorBlueprintResources/StandardMacros.IncrementFloat` _counter
                    (:`  `
                      _))))
              (set `self.Counter` _counter)
              (goto _label)))
          (else
            (goto _label_3)))))
    (else
      (goto _label_2))))

(event `self.PickUp`
  (bind _asfirst_person_character (cast `/Game/FirstPersonBP/Blueprints/FirstPersonCharacter` (`GameplayStatics.GetPlayerCharacter` 0)))
  (set `/Game/FirstPersonBP/Blueprints/FirstPersonCharacter.3Gatling` true _asfirst_person_character)
  (set `/Game/FirstPersonBP/Blueprints/FirstPersonCharacter.AutoFire` true _asfirst_person_character)
  (set `/Game/FirstPersonBP/Blueprints/FirstPersonCharacter.FireRate` 0.1 _asfirst_person_character)
  (`PrimitiveComponent.SetMaterial` (`/Game/FirstPersonBP/Blueprints/FirstPersonCharacter.FP_Gun` _asfirst_person_character) 0 "/Game/FPWeapon/Materials/M_FPGatling.M_FPGatling")
  (`self.K2_DestroyActor`))

(fn `UserConstructionScript`
  (`parent.UserConstructionScript`))